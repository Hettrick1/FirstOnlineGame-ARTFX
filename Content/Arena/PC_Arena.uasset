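; Arena player controller that manages a player's HUD, input state and match-readiness signal.
; On possession it disables pawn input and sets a ready flag through a server event, whose RepNotify asks GS_Arena to check player readiness.
; It also exposes events to build the local HUD with a scoreboard entry per PlayerArray member, toggle input, play a countdown widget and update the health display.
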(event Custom|ChangeInputState
  (params (enable :type Boolean))
  (bind _self self)
  (bind _self_2 self)
  (bind _returnvalue (Pawn|GetControlledPawn _self))
  (if enable
    (Input|EnableInput _returnvalue _self_2)
    (else
      (Input|DisableInput _returnvalue _self_2))))

(event Custom|StartCountdown
  (bind _returnvalue (UserInterface|CreateWidget "/Game/Arena/UI/WBP_Countdown.WBP_Countdown_C"))
  (UserInterface|Viewport|AddtoViewport _returnvalue 0)
  (Default|PlayCountdown _returnvalue))

(event Custom|AddPlayerHUD
  (if (Pawn|IsLocalPlayerController)
    (bind _returnvalue (UserInterface|CreateWidget "/Game/Arena/UI/WBP_PlayerArenaHud.WBP_PlayerArenaHud_C"))
    (bind _output_get (Variables|Default|SethudRef _returnvalue))
    (UserInterface|Viewport|AddtoViewport _output_get 0)
    (for _array_element (Variables|/Script/Engine.GameStateBase|GetPlayerArray (Game|GetGameState))
      (bind _returnvalue_2 (UserInterface|CreateWidget "/Game/Arena/UI/WBP_ScoreBoard.WBP_ScoreBoard_C"))
      (Default|AddPlayertoScoreboard (Variables|Default|GethudRef) _returnvalue_2))))

(event Custom|OnPossesLocal
  (CallFunction|SRVSetIsReady))

(event Custom|SRV_SetIsReady
  (Variables|Default|SetisReady true))

(event Custom|SetPlayerLifePercent
  (params (InPercent :type Float%20%28single-precision%29))
  (Default|SetHealthPercent (Variables|Default|GethudRef) InPercent))

(event EventBeginPlay)

(event EventPossess
  (params (PossessedPawn :type Pawn%20Object%20Reference))
  (CallFunction|ChangeInputState false)
  (CallFunction|OnPossesLocal))

(fn ConstructionScript)

(fn OnRepIsReady
  (bind _asgs_arena (Utilities|Casting|CastToGS_Arena (Game|GetGameState)))
  (Default|CheckIsPlayerReady _asgs_arena))