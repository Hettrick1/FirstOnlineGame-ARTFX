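; GM_Arena is the arena game mode that spawns and possesses a third-person character for each player who logs in.
; On PostLogin it initializes the save system through GI_Game, stopping if that cast fails, and caches all PlayerStart actors if none are stored.
; Each player spawns at the next start in that array, using an incrementing index with no wraparound or bounds check.
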(event EventPostLogin
  (params (NewPlayer :type Player%20Controller%20Object%20Reference))
  (bind _asgi_game (Utilities|Casting|CastToGI_Game (Game|GetGameInstance)))
  (Default|InitializeSaveSystem _asgi_game)
  (if (Utilities|Array|IsEmpty (Variables|Default|GetallPlayerStart))
    (bind _outactors (Actor|GetAllActorsOfClass "/Script/Engine.PlayerStart"))
    (Variables|Default|SetallPlayerStart _outactors))
  (bind _returnvalue (Game|SpawnActorfromClass "/Game/ThirdPerson/Blueprints/BP_ThirdPersonCharacter.BP_ThirdPersonCharacter_C" (Math|Transform|MakeTransform (.location (Transformation|GetActorTransform (Utilities|Array|Get(acopy) (Variables|Default|GetallPlayerStart) (Variables|Default|GetPlayerStartIndex)))) (.rotation (Transformation|GetActorTransform (Utilities|Array|Get(acopy) (Variables|Default|GetallPlayerStart) (Variables|Default|GetPlayerStartIndex)))) "1.000000,1.000000,1.000000") "AdjustIfPossibleButAlwaysSpawn" "MultiplyWithRoot" 0 0))
  (Pawn|Possess NewPlayer _returnvalue)
  (Variables|Default|SetPlayerStartIndex (+ (Variables|Default|GetPlayerStartIndex) 1)))

(fn ConstructionScript)